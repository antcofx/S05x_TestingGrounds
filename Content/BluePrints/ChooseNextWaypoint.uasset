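; Behavior tree task that picks the next patrol waypoint for an AI-controlled ThirdPersonCharacter.
; It reads the pawn's PatrolPoints array and writes the entry at the blackboard Index to the Waypoint key.
; It then advances Index with a modulo wrap so the patrol loops, and finishes successfully.
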(event `self.ReceiveExecuteAI`
  (params (OwnerController :type "AIController Object Reference") (ControlledPawn :type "Pawn Object Reference"))
  (`self.GetControlPoints` ControlledPawn)
  (bind _index (`self.SetNextWayPoint`))
  (`self.CycleIndex` _index)
  (`self.FinishExecute` true))

(fn `CycleIndex`
  (params (A :type Integer))
  (`BTFunctionLibrary.SetBlackboardValueAsInt` (`self.index`) (mod (+ A 1) (`KismetArrayLibrary.Array_Length` (`self.Patrol Points`)))))

(fn `GetControlPoints`
  (params (Object :type "Object Object Reference"))
  (bind _asthird_person_character (cast `/Game/ThirdPersonCPP/Blueprints/ThirdPersonCharacter` Object))
  (set `self.Patrol Points` (`/Game/ThirdPersonCPP/Blueprints/ThirdPersonCharacter.PatrolPoints` _asthird_person_character)))

(fn `SetNextWayPoint`
  (returns (index :type Integer))
  (bind _returnvalue (`BTFunctionLibrary.GetBlackboardValueAsInt` (`self.index`)))
  (`BTFunctionLibrary.SetBlackboardValueAsObject` (`self.Waypoint`) (`KismetArrayLibrary.Array_Get` (`self.Patrol Points`) _returnvalue))
  (return _returnvalue))